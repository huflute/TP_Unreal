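; BP_Cannon_Shoot is a one-shot trigger that fakes a cannon shot with a sound and explosion when the first-person character overlaps it.
; A DoOnce limits each instance to one firing, with the emitter spawned at its Sphere component.
; If FirstActivated is set, a delayed voice line and warning subtitle follow, then the flag is cleared on all instances so later shots skip the reaction.
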(event EventBeginPlay)

(event Collision|EventActorBeginOverlap
  (params (OtherActor :type Actor%20Object%20Reference))
  (Utilities|Casting|CastToFirstPersonCharacter OtherActor)
  (Utilities|FlowControl|DoOnce false
    (:Completed
      (Audio|PlaySound2D "/Game/Audio/SoundCues/SFX/SC_SFX_Cannon_Shoot.SC_SFX_Cannon_Shoot" 1.0 1.0 0.0 0 0)
      (Effects|SpawnEmitteratLocation "/Game/Particles/Explosion/P_Explosion_Big_A.P_Explosion_Big_A" (Transformation|GetWorldLocation (Variables|Default|GetSphere)))
      (if (Variables|Default|GetFirstActivated)
        (Utilities|FlowControl|Delay 1.0)
        (Audio|PlaySound2D "/Game/Audio/Sounds/VOX/MC/VOX_MC_Cannon.VOX_MC_Cannon" 1.0 1.0 0.0 0 0 false)
        (bind _asfirst_person_character (Utilities|Casting|CastToFirstPersonCharacter (Game|GetPlayerCharacter 0)))
        (Default|ChangeSubtitles (Variables|/Game/Blueprints/Player/FirstPersonCharacter.FirstPersonCharacter_C|GetWG_Interface_Ref _asfirst_person_character) "Wow ! I should be careful around those !" 4.0 false)
        (bind _outactors (Actor|GetAllActorsOfClass "BP_Cannon_Shoot_C"))
        (for _array_element _outactors
          (Variables|BP_Cannon_Shoot_C|SetFirstActivated _array_element false))))))

(event EventTick
  (params (DeltaSeconds :type Float%20%28single-precision%29)))

(fn ConstructionScript)