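; Ending-sequence actor that plays the closing treasure dialogue and then quits the game.
; EndDialogue disables player input, pushes the Cinematic sound mix and plays each voice line with matching subtitles on the first-person character's UI, using a delayed loop timed to each sound's duration.
; Ambience fades in during the dialogue and out afterwards, followed by a camera shake, fade sequence and volcano eruption sound before quitting.
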(event Custom|EndDialogue
  (Input|DisableInput (Game|GetPlayerCharacter 0) (Game|GetPlayerController 0))
  (Audio|PushSoundMixModifier "/Game/Audio/SoundClass/SCMix/Cinematic.Cinematic")
  (Utilities|FlowControl|Delay 1.0)
  (bind _asfirst_person_character (Utilities|Casting|CastToFirstPersonCharacter (Game|GetPlayerCharacter 0)))
  (bind (_arrayelement _arrayindex) (Utilities|ForEachLoopwithDelay (Variables|Default|GetEndDialogues) (+ (Variables|/Script/Engine.SoundBase|GetDuration (stale _arrayelement)) 0.5))
    (:LoopBody
      (Audio|PlaySound2D _arrayelement 1.0 1.0 0.0 0 0)
      (Default|ChangeSubtitles (Variables|/Game/Blueprints/Player/FirstPersonCharacter.FirstPersonCharacter_C|GetWG_Interface_Ref _asfirst_person_character) (Utilities|Array|Get(acopy) (Variables|Default|GetEndSubtitles) _arrayindex) (+ (Variables|/Script/Engine.SoundBase|GetDuration _arrayelement) 0.5) true)
      (if (== _arrayindex 1)
        (Audio|Components|Audio|FadeIn (Variables|Default|GetAMB) 0.5 1.0 0.0 "Linear" :!class /Script/Engine.AudioComponent)))
    (:Completed
      (Audio|Components|Audio|FadeOut (Variables|Default|GetAMB) 0.5 0.0 "Linear" :!class /Script/Engine.AudioComponent)
      (Camera|PlayWorldCameraShake "/Game/Blueprints/Camera/BP_EndCameraShake.BP_EndCameraShake_C" (Transformation|GetActorLocation (Game|GetPlayerCharacter 0)) 0.0 2e+02)
      (Sequencer|Player|Play (Variables|/Script/LevelSequence.LevelSequenceActor|GetSequencePlayer (Variables|Default|GetFadeSequence)) :!class /Script/MovieScene.MovieSceneSequencePlayer)
      (Audio|PlaySound2D "/Game/Audio/SoundCues/SFX/Gameplay/SC_SFX_Volcano_Eruption.SC_SFX_Volcano_Eruption" 1.0 1.0 0.0 0 0)
      (Utilities|FlowControl|Delay 1e+01)
      (Game|QuitGame (Game|GetPlayerController 0) "Quit" true))))

(event EventBeginPlay)

(event Collision|EventActorBeginOverlap
  (params (OtherActor :type Actor%20Object%20Reference)))

(event EventTick
  (params (DeltaSeconds :type Float%20%28single-precision%29)))

(fn ConstructionScript)