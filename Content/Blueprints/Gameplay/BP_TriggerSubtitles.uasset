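; BP_TriggerSubtitles is a trigger box that plays a one-shot voice line with on-screen subtitles when the first-person character overlaps it.
; If the Manager is already speaking, it first delays by half its own line's duration.
; It then sends text to the character's widget, plays the 2D sound, deactivates itself, and holds the Manager's IsSpeaking flag until the line's duration elapses.
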(event OnComponentBeginOverlap(Box)
  (params (OverlappedComponent :type Primitive%20Component%20Object%20Reference) (OtherActor :type Actor%20Object%20Reference) (OtherComp :type Primitive%20Component%20Object%20Reference) (OtherBodyIndex :type Integer) (bFromSweep :type Boolean) (SweepResult :type Hit%20Result%20Structure%20%28by%20ref%29))
  (bind _linetoplay (Variables|Default|GetLineToPlay))
  (bind _duration (Variables|/Script/Engine.SoundBase|GetDuration _linetoplay))
  (if (Variables|Default|GetActive?)
    (Variables|Default|SetTriggered true)
    (if (Variables|/Game/Blueprints/Sound/BP_Dialogue_Manager.BP_Dialogue_Manager_C|GetIsSpeaking (Variables|Default|GetManager))
      (Utilities|FlowControl|DoOnce false
        (:Completed
          (Utilities|FlowControl|Delay (- _duration (/ _duration 2.0)))))
      (else
        (Utilities|FlowControl|DoOnce false
          (:Completed
            _))))
    (bind _asfirst_person_character (Utilities|Casting|CastToFirstPersonCharacter OtherActor))
    (Default|ChangeSubtitles (Variables|/Game/Blueprints/Player/FirstPersonCharacter.FirstPersonCharacter_C|GetWG_Interface_Ref _asfirst_person_character) (Variables|Default|GetSubtitles_Text) (Variables|Default|GetSubtitles_ScreenTime) false)
    (Variables|/Game/Blueprints/Sound/BP_Dialogue_Manager.BP_Dialogue_Manager_C|SetIsSpeaking (Variables|Default|GetManager) true)
    (Audio|PlaySound2D (Variables|Default|GetLineToPlay) 1.0 1.0 0.0 0 0)
    (Variables|Default|SetActive? false)
    (Utilities|FlowControl|Delay (Variables|/Script/Engine.SoundBase|GetDuration (Variables|Default|GetLineToPlay)))
    (Variables|/Game/Blueprints/Sound/BP_Dialogue_Manager.BP_Dialogue_Manager_C|SetIsSpeaking (Variables|Default|GetManager) false)))

(event Collision|EventActorBeginOverlap
  (params (OtherActor :type Actor%20Object%20Reference)))

(event EventTick
  (params (DeltaSeconds :type Float%20%28single-precision%29)))

(fn ConstructionScript)