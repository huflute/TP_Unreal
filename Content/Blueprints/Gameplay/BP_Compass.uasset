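; BP_Compass is a collectible compass pickup that counts toward unlocking a door.
; Each tick it makes its mesh visible once its linked Trigger reports triggered, which happens after the player steps on the door.
; Interacting increments the Door's compass count, has the Door check it against its maximum, and destroys the compass.
; An Outline event toggles custom depth stencil rendering to highlight the mesh.
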(event Collision|EventActorBeginOverlap
  (params (OtherActor :type Actor%20Object%20Reference)))

(event EventTick
  (params (DeltaSeconds :type Float%20%28single-precision%29))
  ;[1 1 1] Fait apparaître les boussoles quand on a marché sur la porte
  (if (Variables|/Game/Blueprints/Gameplay/BP_TriggerSubtitles.BP_TriggerSubtitles_C|GetTriggered (Variables|Default|GetTrigger))
    (Rendering|SetVisibility (Variables|Default|GetSM_PirateCompass_1) true false)))

(event EventOutline
  (params (On? :type Boolean))
  (bind _sm_piratecompass_1 (Variables|Default|GetSM_PirateCompass_1))
  (Rendering|SetRenderCustomDepth _sm_piratecompass_1 On?)
  (Rendering|SetCustomDepthStencilValue _sm_piratecompass_1 2))

(event EventInteract
  (params (ShotInteract? :type Boolean))
  (bind _door (Variables|Default|GetDoor))
  ;[1 1 1] Ramasse la boussole et incrémente le compass counter
  (bind _result (Math|Integer|IncrementInt (Variables|/Game/Blueprints/Gameplay/BP_Boat_Door.BP_Boat_Door_C|GetCompass (Variables|Default|GetDoor)))
    (:%20%20
      (Default|CheckCompass _door _result (Variables|/Game/Blueprints/Gameplay/BP_Boat_Door.BP_Boat_Door_C|GetMaxCompass _door))
      (Actor|DestroyActor self))))

(fn ConstructionScript)