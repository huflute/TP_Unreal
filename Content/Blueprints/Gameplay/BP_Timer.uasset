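; BP_Timer is a countdown timer actor that quits the game when minutes and seconds run out.
; While CountdownTrigger's Active flag is false, Tick shows the WG_Timer widget once through a DoOnce and feeds a one-second Delay.
; The Delay ignores calls while pending, so it paces the per-frame Tick into a once-per-second decrement that rolls Seconds over into Minutes.
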(event EventBeginPlay)

(event Collision|EventActorBeginOverlap
  (params (OtherActor :type Actor%20Object%20Reference)))

(event EventTick
  (params (DeltaSeconds :type Float%20%28single-precision%29))
  (if (not (Variables|/Game/Blueprints/Gameplay/BP_TriggerDialogue.BP_TriggerDialogue_C|GetActive? (Variables|Default|GetCountdownTrigger)))
    (Utilities|FlowControl|Sequence
      (:then_0
        (Utilities|FlowControl|DoOnce false
          (:Completed
            (bind _returnvalue (UserInterface|CreateWidget "/Game/Blueprints/UI/WG_Timer.WG_Timer_C"))
            (UserInterface|Viewport|AddtoViewport _returnvalue 0))))
      (:then_1
        (Utilities|FlowControl|Delay 1.0)
        (if (== (Variables|Default|GetSeconds) 0)
          (if (== (Variables|Default|GetMinutes) 0)
            (Game|QuitGame (Game|GetPlayerController 0) "Quit" true)
            (else
              (Variables|Default|SetSeconds 59)
              (Math|Integer|DecrementInt (Variables|Default|GetMinutes))))
          (else
            (Math|Integer|DecrementInt (Variables|Default|GetSeconds))))))))

(fn ConstructionScript)