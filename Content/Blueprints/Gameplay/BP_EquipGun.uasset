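; BP_EquipGun is a trigger box that equips the player's weapon and plays an accompanying voice line.
; While Active, an overlap shows a subtitle through the character's UI and plays the optional 2D line, setting the Manager's IsSpeaking flag for its duration.
; If speech is already running, the line first waits half its own length.
; The trigger equips the gun and deactivates itself without waiting for audio.
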(event OnComponentBeginOverlap(Box)
  (params (OverlappedComponent :type Primitive%20Component%20Object%20Reference) (OtherActor :type Actor%20Object%20Reference) (OtherComp :type Primitive%20Component%20Object%20Reference) (OtherBodyIndex :type Integer) (bFromSweep :type Boolean) (SweepResult :type Hit%20Result%20Structure%20%28by%20ref%29))
  (bind _linetoplay (Variables|Audio|GetLineToPlay))
  (bind _duration (Variables|/Script/Engine.SoundBase|GetDuration _linetoplay))
  (if (Variables|Default|GetActive?)
    (Utilities|FlowControl|Sequence
      (:then_0
        (if (Variables|/Game/Blueprints/Sound/BP_Dialogue_Manager.BP_Dialogue_Manager_C|GetIsSpeaking (Variables|Audio|GetManager))
          (Utilities|FlowControl|DoOnce false
            (:Completed
              (Utilities|FlowControl|Delay (- _duration (/ _duration 2.0)))))
          (else
            (Utilities|FlowControl|DoOnce false
              (:Completed
                _))))
        (bind _asfirst_person_character (Utilities|Casting|CastToFirstPersonCharacter OtherActor))
        (Default|ChangeSubtitles (Variables|/Game/Blueprints/Player/FirstPersonCharacter.FirstPersonCharacter_C|GetWG_Interface_Ref _asfirst_person_character) (Variables|Text|GetSubtitles_Text) (Variables|Text|GetSubtitles_ScreenTime) false)
        (Utilities|IsValid (Variables|Audio|GetLineToPlay)
          (:Is%20Valid
            (Variables|/Game/Blueprints/Sound/BP_Dialogue_Manager.BP_Dialogue_Manager_C|SetIsSpeaking (Variables|Audio|GetManager) true)
            (Audio|PlaySound2D (Variables|Audio|GetLineToPlay) 1.0 1.0 0.0 0 0)
            (Utilities|FlowControl|Delay (Variables|/Script/Engine.SoundBase|GetDuration (Variables|Audio|GetLineToPlay)))
            (Variables|/Game/Blueprints/Sound/BP_Dialogue_Manager.BP_Dialogue_Manager_C|SetIsSpeaking (Variables|Audio|GetManager) false))))
      (:then_1
        (bind _asfirst_person_character_2 (Utilities|Casting|CastToFirstPersonCharacter (Game|GetPlayerCharacter 0)))
        (Default|EquipWeapon _asfirst_person_character_2))
      (:then_2
        (Variables|Default|SetActive? false)))))

(event Collision|EventActorBeginOverlap
  (params (OtherActor :type Actor%20Object%20Reference)))

(event EventTick
  (params (DeltaSeconds :type Float%20%28single-precision%29)))

(fn ConstructionScript)